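; BP_Inventory is the player inventory Blueprint, which maps Enhanced Input actions to inventory UI and hotbar controls.
; The toggle action shows or hides the inventory UI, while slot keys set the selected hotbar index and next/previous actions cycle through it.
; BeginPlay binds an empty initialization event as a hook for custom setup.
; Additional hotbar keys also need registering in the component's Select Index input action array.
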(event Custom|OnInventoryInitialized_Event
  ;[1 1 1] In case you want to do anything on Inventory's initialization
)

(event Input|EnhancedActionEvents|EnhancedInputActionIA_NextIndex
  (params (ActionValue :type Boolean) (ElapsedSeconds :type Float%20%28double-precision%29) (TriggeredSeconds :type Float%20%28double-precision%29) (InputAction :type Input%20Action%20Object%20Reference :default "/InventorySystem/Input/IA_NextIndex.IA_NextIndex"))
  ;[1 1 1] Basic Input
  (:Completed
    (Class|PlayerInventoryBase|SelectNextHotbarItem)))

(event Input|EnhancedActionEvents|EnhancedInputActionIA_SelectSlot1
  (params (ActionValue :type Boolean) (ElapsedSeconds :type Float%20%28double-precision%29) (TriggeredSeconds :type Float%20%28double-precision%29) (InputAction :type Input%20Action%20Object%20Reference :default "/InventorySystem/Input/SelectHotbarSlot/IA_SelectSlot1.IA_SelectSlot1"))
  ;[1 0.6822 0] Hotbar keys. If you want to add more make sure you add the Input Actions to the Select Index Input Action Array. (In Class Defaults or in the instantiated Inventory component itself)
  (:Completed
    (Class|PlayerInventoryBase|SetSelectedIndex)))

(event Input|EnhancedActionEvents|EnhancedInputActionIA_PrevIndex
  (params (ActionValue :type Boolean) (ElapsedSeconds :type Float%20%28double-precision%29) (TriggeredSeconds :type Float%20%28double-precision%29) (InputAction :type Input%20Action%20Object%20Reference :default "/InventorySystem/Input/IA_PrevIndex.IA_PrevIndex"))
  ;[1 1 1] Basic Input
  (:Completed
    (Class|PlayerInventoryBase|SelectPreviousHotbarItem)))

(event Input|EnhancedActionEvents|EnhancedInputActionIA_ToggleInventory
  (params (ActionValue :type Boolean) (ElapsedSeconds :type Float%20%28double-precision%29) (TriggeredSeconds :type Float%20%28double-precision%29) (InputAction :type Input%20Action%20Object%20Reference :default "/InventorySystem/Input/IA_ToggleInventory.IA_ToggleInventory"))
  ;[1 1 1] Basic Input
  (:Completed
    (Default|ToggleVisiblityEvent (Variables|Default|GetInventoryUI))))

(event Input|EnhancedActionEvents|EnhancedInputActionIA_SelectSlot2
  (params (ActionValue :type Boolean) (ElapsedSeconds :type Float%20%28double-precision%29) (TriggeredSeconds :type Float%20%28double-precision%29) (InputAction :type Input%20Action%20Object%20Reference :default "/InventorySystem/Input/SelectHotbarSlot/IA_SelectSlot2.IA_SelectSlot2"))
  ;[1 0.6822 0] Hotbar keys. If you want to add more make sure you add the Input Actions to the Select Index Input Action Array. (In Class Defaults or in the instantiated Inventory component itself)
  (:Completed
    (Class|PlayerInventoryBase|SetSelectedIndex 1)))

(event Input|EnhancedActionEvents|EnhancedInputActionIA_SelectSlot3
  (params (ActionValue :type Boolean) (ElapsedSeconds :type Float%20%28double-precision%29) (TriggeredSeconds :type Float%20%28double-precision%29) (InputAction :type Input%20Action%20Object%20Reference :default "/InventorySystem/Input/SelectHotbarSlot/IA_SelectSlot3.IA_SelectSlot3"))
  ;[1 0.6822 0] Hotbar keys. If you want to add more make sure you add the Input Actions to the Select Index Input Action Array. (In Class Defaults or in the instantiated Inventory component itself)
  (:Completed
    (Class|PlayerInventoryBase|SetSelectedIndex 2)))

(event EventBeginPlay
  ;[1 1 1] In case you want to do anything on Inventory's initialization
  (EventDispatchers|AssignOnInventoryInitialized (delegate Custom|OnInventoryInitialized_Event)))